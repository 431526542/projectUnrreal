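; AI controller for the BadGay1 enemy that runs behavior tree BBT_BadGay1 on possess and feeds player detection into its blackboard.
; Sensing the player cancels the lose-sight timer and sets HasLineofSight, but the node storing EnemyActor is disconnected.
; Other perception updates set that timer with zero time, so it never fires.
; Its handler would clear EnemyActor yet sets HasLineofSight true, not false.
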(event `self.ReceivePossess`
  (params (PossessedPawn :type "Pawn Object Reference"))
  (`self.RunBehaviorTree` "/Game/MyPown/MyPown/BadGay1/BBT_BadGay1.BBT_BadGay1"))

(event `self.AIPerception.OnTargetPerceptionUpdated`
  (params (Actor :type "Actor Object Reference") (Stimulus :type "AIStimulus Structure"))
  (if (and (== Actor (`GameplayStatics.GetPlayerCharacter` 0)) (`.bSuccessfullySensed` (break `AIStimulus` Stimulus)))
    (`KismetSystemLibrary.K2_ClearAndInvalidateTimerHandle` (`self.EnemyHandle`))
    (`BlackboardComponent.SetValueAsBool` (`self.Blackboard`) (`self.HasLineofSight`) true)
    (else
      (bind _returnvalue (`KismetSystemLibrary.K2_SetTimerDelegate` (delegate `EnemyTimer`)))
      (set `self.EnemyHandle` _returnvalue))))

(event `EnemyTimer`
  (bind _blackboard (`self.Blackboard`))
  (`BlackboardComponent.SetValueAsBool` _blackboard (`self.HasLineofSight`) true)
  (`BlackboardComponent.SetValueAsObject` _blackboard (`self.EnemyActor`) null))

(fn `UserConstructionScript`)