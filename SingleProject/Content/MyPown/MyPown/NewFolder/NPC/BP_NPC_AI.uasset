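; BP_NPC_AI is the AI controller that runs the BT_NPC behavior tree for patrolling, investigating NPCs.
; On BeginPlay it seeds the blackboard with the pawn's patrol path looping and wait settings plus an initial direction.
; Perception updates pass stimuli to ComplateSenses, which branches on array index as sense type.
; The first sets CanSeePlayer; successful second or third senses set investigation state and target location, the second also playing a sound.
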(event `self.ReceiveBeginPlay`
  (bind _returnvalue (`AIBlueprintHelperLibrary.GetBlackboard` null))
  (`self.RunBehaviorTree` "/Game/MyPown/MyPown/NewFolder/NPC/BT_NPC.BT_NPC")
  ;[1 1 1] 루핑코드에 관련된 것
  (bind _asbp_npc (cast `/Game/MyPown/MyPown/NewFolder/NPC/BP_NPC` (`self.K2_GetPawn`)))
  (bind _output_get (set `self.MyPawn` _asbp_npc))
  (`BlackboardComponent.SetValueAsBool` (`AIBlueprintHelperLibrary.GetBlackboard` null) "PathLooping" (`/Game/MyPown/MyPown/NewFolder/NPC/PatrollPart.IsLooping` (`/Game/MyPown/MyPown/NewFolder/NPC/BP_NPC.PatrollPath` _output_get)))
  (`BlackboardComponent.SetValueAsInt` _returnvalue "Direction" 1)
  (`BlackboardComponent.SetValueAsFloat` _returnvalue "WaitTime" (`/Game/MyPown/MyPown/NewFolder/NPC/PatrollPart.WaitTime` (`/Game/MyPown/MyPown/NewFolder/NPC/BP_NPC.PatrollPath` (`self.MyPawn`)))))

(event `self.AIPerception.OnPerceptionUpdated`
  (params (UpdatedActors :type "Array of Actor Object Reference (by ref)"))
  (for _array_element UpdatedActors
    (bind _info (`AIPerceptionComponent.GetActorsPerception` (`self.AIPerception`) _array_element))
    (`self.ComplateSenses` (`.LastSensedStimuli` (break `ActorPerceptionBlueprintInfo` _info)))))

(fn `ComplateSenses`
  (params (Array :type "Array of AIStimulus Structure"))
  (bind (_local_senes_age _local_senes_expirationage _local_senes_strength _local_senes_stimuluslocation _local_senes_receiverlocation _local_senes_tag _local_senes_bsuccessfullysensed) (break `AIStimulus` (`self.Local_Senes`)))
  (bind (_local_senes_age_2 _local_senes_expirationage_2 _local_senes_strength_2 _local_senes_stimuluslocation_2 _local_senes_receiverlocation_2 _local_senes_tag_2 _local_senes_bsuccessfullysensed_2) (break `AIStimulus` (`self.Local_Senes`)))
  (for (_array_element _array_index) Array
    (set `self.Local_Senes` _array_element)
    (switch `int` _array_index
      (:`0`
        (`BlackboardComponent.SetValueAsBool` (`AIBlueprintHelperLibrary.GetBlackboard` null) "CanSeePlayer" _local_senes_bsuccessfullysensed))
      (:`1`
        (if _local_senes_bsuccessfullysensed
          (`GameplayStatics.PlaySoundAtLocation` "/Game/StarterContent/Audio/Steam01_Cue.Steam01_Cue" _local_senes_receiverlocation (struct) 1.0 1.0 0.0 null null null)
          (`BlackboardComponent.SetValueAsBool` (`AIBlueprintHelperLibrary.GetBlackboard` null) "IsInvestigating" _local_senes_bsuccessfullysensed_2 :!label _label)
          (`BlackboardComponent.SetValueAsVector` (`AIBlueprintHelperLibrary.GetBlackboard` null) "TargetLocation" _local_senes_stimuluslocation_2)))
      (:`2`
        (if _local_senes_bsuccessfullysensed
          (goto _label))))))

(fn `UserConstructionScript`)