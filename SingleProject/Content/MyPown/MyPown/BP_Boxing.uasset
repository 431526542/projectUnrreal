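; BP_Boxing is a player-controlled boxer with movement, look and four punch attacks.
; Axis inputs move it along the control rotation's forward and right vectors and drive yaw and pitch.
; Jab, straight, left hook and right hook inputs each play a montage on the Mesh behind their own DoOnce, reset only on montage completion.
; The gates are independent, so none blocks a different punch.
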(event `InputAxis|MoveForward`
  (params (AxisValue :type "Float (single-precision)"))
  ;[1 1 1] 이동
  (`self.AddMovementInput` (`KismetMathLibrary.GetForwardVector` (`self.GetControlRotation`)) AxisValue))

(event `InputAxis|Turn`
  (params (AxisValue :type "Float (single-precision)"))
  ;[1 1 1] 이동
  (`self.AddControllerYawInput` AxisValue))

(event `InputAxis|LookUp`
  (params (AxisValue :type "Float (single-precision)"))
  ;[1 1 1] 이동
  (`self.AddControllerPitchInput` AxisValue))

(event `InputAxis|MoveRight`
  (params (AxisValue :type "Float (single-precision)"))
  ;[1 1 1] 이동
  (`self.AddMovementInput` (`KismetMathLibrary.GetRightVector` (`self.GetControlRotation`)) AxisValue))

(event `InputAction|Attack1`
  (params (Key :type "Key Structure"))
  ;[1 1 1] 공격
  (:`Pressed`
    (`/Engine/EditorBlueprintResources/StandardMacros.DoOnce` false :!label _label
      (:`Completed`
        (`|PlayMontage` (`self.Mesh`) "/Game/MyPown/MyPown/Boxing/Boxing_Jap_Montage.Boxing_Jap_Montage"
          (:`OnCompleted`
            (goto _label :!via `Reset`)))))))

(event `InputAction|Attack2`
  (params (Key :type "Key Structure"))
  ;[1 1 1] 공격
  (:`Pressed`
    (`/Engine/EditorBlueprintResources/StandardMacros.DoOnce` false :!label _label_2
      (:`Completed`
        (`|PlayMontage` (`self.Mesh`) "/Game/MyPown/MyPown/Boxing/Boxing_Straight_Montage.Boxing_Straight_Montage"
          (:`OnCompleted`
            (goto _label_2 :!via `Reset`)))))))

(event `InputAction|LeftHook`
  (params (Key :type "Key Structure"))
  ;[1 1 1] 공격
  (:`Pressed`
    (`/Engine/EditorBlueprintResources/StandardMacros.DoOnce` false :!label _label_3
      (:`Completed`
        (`|PlayMontage` (`self.Mesh`) "/Game/MyPown/MyPown/Boxing/LeftHook_Montage.LeftHook_Montage"
          (:`OnCompleted`
            (goto _label_3 :!via `Reset`)))))))

(event `InputAction|RigthHook`
  (params (Key :type "Key Structure"))
  ;[1 1 1] 공격
  (:`Pressed`
    (`/Engine/EditorBlueprintResources/StandardMacros.DoOnce` false :!label _label_4
      (:`Completed`
        (`|PlayMontage` (`self.Mesh`) "/Game/MyPown/MyPown/Boxing/RightHook_Montage.RightHook_Montage"
          (:`OnCompleted`
            (goto _label_4 :!via `Reset`)))))))

(fn `UserConstructionScript`)