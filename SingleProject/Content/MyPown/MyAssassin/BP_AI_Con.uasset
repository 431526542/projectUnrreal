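; BP_AI_Con is an AI controller that runs the BT_AI behavior tree on possession and tracks the player through AI perception.
; A successful sighting of the player cancels any pending forget timer and writes HasLineofSight and EnemyActor to the Blackboard.
; Any other perception update starts a four-second one-shot timer that clears both keys, giving the AI a short memory before it drops the target.
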(event `self.ReceivePossess`
  (params (PossessedPawn :type "Pawn Object Reference"))
  (`self.RunBehaviorTree` "/Game/MyPown/MyAssassin/BT_AI.BT_AI"))

(event `self.AIPerception.OnTargetPerceptionUpdated`
  (params (Actor :type "Actor Object Reference") (Stimulus :type "AIStimulus Structure"))
  (bind _blackboard (`self.Blackboard`))
  (if (and (== Actor (`GameplayStatics.GetPlayerCharacter` 0)) (`.bSuccessfullySensed` (break `AIStimulus` Stimulus)))
    (`KismetSystemLibrary.K2_ClearAndInvalidateTimerHandle` (`self.Enemy Handle`))
    (`BlackboardComponent.SetValueAsBool` _blackboard (`self.HasLineofSight`) true)
    (`BlackboardComponent.SetValueAsObject` _blackboard (`self.EnemyActor`) Actor)
    (else
      (bind _returnvalue (`KismetSystemLibrary.K2_SetTimerDelegate` (delegate `EnemyTimer`) 4.0))
      (set `self.Enemy Handle` _returnvalue))))

(event `EnemyTimer`
  (bind _blackboard (`self.Blackboard`))
  (`BlackboardComponent.SetValueAsBool` _blackboard (`self.HasLineofSight`) false)
  (`BlackboardComponent.SetValueAsObject` _blackboard (`self.EnemyActor`) null))

(fn `UserConstructionScript`)