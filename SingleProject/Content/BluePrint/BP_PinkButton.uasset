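; BP_PinkButton is a button actor that sets a group of pink blocks moving when activated.
; Its PinkButton_event spawns an explosion emitter at the button, plays a 2D button sound, then calls PinkBlockMoveEvent on eight referenced block variables.
; The event has no trigger within this Blueprint, as BeginPlay, overlap and Tick are empty.
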(event `PinkButton_event`
  (`GameplayStatics.SpawnEmitterAtLocation` "/Game/StarterContent/Particles/P_Explosion.P_Explosion" (`self.K2_GetActorLocation`))
  (`GameplayStatics.PlaySound2D` "/Game/MySound/L1_Button_Cue.L1_Button_Cue" 1.0 1.0 0.0 null null)
  (`/Game/BP_block/BP_L1Pink.PinkBlockMove_event` (`self.L1PinkBluck`))
  (`/Game/BP_block/BP_L1Pink.PinkBlockMove_event` (`self.NewVar_1`))
  (`/Game/BP_block/BP_L1Pink.PinkBlockMove_event` (`self.NewVar_2`))
  (`/Game/BP_block/BP_L1Pink.PinkBlockMove_event` (`self.NewVar_3`))
  (`/Game/BP_block/BP_L1Pink.PinkBlockMove_event` (`self.NewVar_4`))
  (`/Game/BP_block/BP_L1Pink.PinkBlockMove_event` (`self.NewVar_5`))
  (`/Game/BP_block/BP_L1Pink.PinkBlockMove_event` (`self.NewVar_6`))
  (`/Game/BP_block/BP_L1Pink.PinkBlockMove_event` (`self.NewVar_7`)))

(fn `UserConstructionScript`)