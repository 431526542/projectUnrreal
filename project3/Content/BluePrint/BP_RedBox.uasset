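; BP_RedBox is a clickable cube that turns redder with each click and finally explodes.
; Each click writes the Plus1 counter into the green and blue channels of the Color material parameter, then lowers it by a fixed step.
; When Plus1 reaches the low threshold, it spawns an explosion emitter at the cube and destroys only the Cube component, not the actor.
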(event `self.Cube.OnClicked`
  (params (TouchedComponent :type "PrimitiveComponent Object Reference") (ButtonPressed :type "Key Structure"))
  (bind _plus1 (`self.Plus1`))
  (bind _plus1_2 (`self.Plus1`))
  (`MeshComponent.SetVectorParameterValueOnMaterials` (`self.Cube`) "Color" (`KismetMathLibrary.MakeVector` 1.0 _plus1_2 _plus1_2))
  (if (>= 0.1 _plus1)
    (`GameplayStatics.SpawnEmitterAtLocation` "/Game/StarterContent/Particles/P_Explosion.P_Explosion" (`SceneComponent.K2_GetComponentLocation` (`self.Cube`)))
    (`ActorComponent.K2_DestroyComponent` (`self.Cube`))
    (else
      (set `self.Plus1` (- _plus1 0.1)))))

(fn `UserConstructionScript`)