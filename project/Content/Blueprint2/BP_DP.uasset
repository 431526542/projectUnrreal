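; BP_DP is a click-to-destroy Blueprint that removes BP_Sphere objects the player aims at.
; On a left mouse press, it line traces 10000 units on the Visibility channel along the player camera's forward vector.
; If the hit actor casts to BP_Sphere, that actor is destroyed.
; BeginPlay, Tick, overlap and the construction script hold no logic.
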(event `Key|LeftMouseButton`
  (params (Key :type "Key Structure"))
  (bind _returnvalue (`GameplayStatics.GetPlayerCameraManager` 0))
  (bind _returnvalue_2 (`PlayerCameraManager.GetCameraLocation` _returnvalue))
  (:`Pressed`
    (bind (_outhit _returnvalue_3) (`KismetSystemLibrary.LineTraceSingle` _returnvalue_2 (+ (* (`KismetMathLibrary.GetForwardVector` (`PlayerCameraManager.GetCameraRotation` _returnvalue)) 10000.0) _returnvalue_2) "TraceTypeQuery1"))
    (if _returnvalue_3
      (bind _asbp_sphere (cast `/Game/Blueprint2/BP_Sphere` (`.HitActor` (`GameplayStatics.BreakHitResult` _outhit))))
      (`self.K2_DestroyActor` _asbp_sphere))))

(fn `UserConstructionScript`)